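; Desk fan actor that runs only while the generator is on.
; On BeginPlay it gets the generator through the player character's Enemy reference.
; Tick polls the generator's ON state, and two DoOnce gates that reset each other make the Fan component play or stop once per power change.
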(event `self.ReceiveBeginPlay`
  (bind _as0_base_human (cast `/Game/Blueprints/Characters/0_Base_Human` (`GameplayStatics.GetPlayerCharacter` 0)))
  (set `self.Generator` (`/Game/Blueprints/SoulanityBPs/Enemy/Enemy.Generator` (`/Game/Blueprints/Characters/0_Base_Human.Enemy` _as0_base_human))))

(event `self.ReceiveTick`
  (params (DeltaSeconds :type "Float (single-precision)"))
  (bind _fan (`self.Fan`))
  (if (`/Game/Blueprints/SoulanityBPs/Items/Light_Items/Light_Trigger.ON?` (`self.Generator`))
    (`/Engine/EditorBlueprintResources/StandardMacros.DoOnce` false :!label _label
      (:`Completed`
        (`SkeletalMeshComponent.Play` _fan true)
        (goto _label_2 :!via `Reset`)))
    (else
      (`/Engine/EditorBlueprintResources/StandardMacros.DoOnce` false :!label _label_2
        (:`Completed`
          (`SkeletalMeshComponent.Stop` _fan)
          (goto _label :!via `Reset`))))))

(fn `UserConstructionScript`)