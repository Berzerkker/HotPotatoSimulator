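; Sanity potion pickup actor that restores the player's Sanity, capped at 100, and destroys itself when used.
; Overlap with a human in the detection zone enables input, prints a prompt and opens a Gate that E passes through and Q closes; leaving disables input.
; A delayed Tick replays a timeline that pulses the mesh's glow, creating a dynamic material instance on each update.
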(event `Key|E`
  (params (Key :type "Key Structure"))
  (:`Pressed`
    (`/Engine/EditorBlueprintResources/StandardMacros.Gate` true :!label _label
      (:`Exit`
        (bind _ashuman (cast `/Game/Blueprints/Characters/Human` (`GameplayStatics.GetPlayerCharacter` 0)))
        (bind _output_get (set `self.PlayerObject` _ashuman))
        (bind _output_get_2 (set `/Game/Blueprints/Characters/0_Base_Human.Sanity` (+ (`/Game/Blueprints/Characters/0_Base_Human.Sanity` (`self.PlayerObject`)) 30.0) _output_get))
        (if (> _output_get_2 100.0)
          (set `/Game/Blueprints/Characters/0_Base_Human.Sanity` 100.0 (`self.PlayerObject`))
          (`self.K2_DestroyActor`)
          (else
            (`self.K2_DestroyActor`)))))))

(event `self.DetectionZone.OnComponentBeginOverlap`
  (params (OverlappedComponent :type "PrimitiveComponent Object Reference") (OtherActor :type "Actor Object Reference") (OtherComp :type "PrimitiveComponent Object Reference") (OtherBodyIndex :type Integer) (bFromSweep :type Boolean) (SweepResult :type "HitResult Structure (by ref)"))
  (cast `/Game/Blueprints/Characters/0_Base_Human` OtherActor)
  (`self.EnableInput` (`GameplayStatics.GetPlayerController` 0))
  (`KismetSystemLibrary.PrintString` "Press E to pick up potion")
  (goto _label :!via `Open`))

(event `Key|Q`
  (params (Key :type "Key Structure"))
  (:`Pressed`
    (goto _label :!via `Close`)))

(event `self.DetectionZone.OnComponentEndOverlap`
  (params (OverlappedComponent :type "PrimitiveComponent Object Reference") (OtherActor :type "Actor Object Reference") (OtherComp :type "PrimitiveComponent Object Reference") (OtherBodyIndex :type Integer))
  (cast `/Game/Blueprints/Characters/0_Base_Human` OtherActor)
  (`self.DisableInput` (`GameplayStatics.GetPlayerController` 0)))

(event `self.ReceiveTick`
  (params (DeltaSeconds :type "Float (single-precision)"))
  (`KismetSystemLibrary.Delay` 5.0)
  (bind (_direction _newtrack_0) (`Timeline|Timeline_0` :!via `PlayFromStart`)
    (:`Update`
      (bind _returnvalue (`PrimitiveComponent.CreateDynamicMaterialInstance` (`self.StaticMesh`) 0 "/Game/Meshes/SanityPotionPickup/SanityPotion_Pickup_Mat_Inst.SanityPotion_Pickup_Mat_Inst"))
      (`MaterialInstanceDynamic.SetScalarParameterValue` _returnvalue "GlowIntensity" _newtrack_0))))

(fn `UserConstructionScript`)