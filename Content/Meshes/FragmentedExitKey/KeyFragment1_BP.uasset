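; Pickup actor for a fragment of the exit key, collected by the player.
; A Sphere overlap with a 0_Base_Human shows a prompt, enables input and opens a gate, and leaving reverses the input and gate.
; Pressing E or Q through the open gate increments KeySectionsFound on GameplayGM while below three, has the game mode spawn a key fragment, then destroys the actor.
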(event `Key|E`
  (params (Key :type "Key Structure"))
  (:`Pressed`
    (`/Engine/EditorBlueprintResources/StandardMacros.Gate` true :!label _label
      (:`Exit`
        (bind _asgameplay_gm (cast `/Game/Blueprints/Gameplay/GameplayGM` (`GameplayStatics.GetGameMode`)))
        (bind _keysectionsfound (`/Game/Blueprints/Gameplay/GameplayGM.KeySectionsFound` _asgameplay_gm))
        (if (not (>= _keysectionsfound 3))
          (set `/Game/Blueprints/Gameplay/GameplayGM.KeySectionsFound` (+ _keysectionsfound 1) _asgameplay_gm)
          (`/Game/Blueprints/Gameplay/GameplayGM.Spawn A Key Fragment` _asgameplay_gm)
          (`KismetSystemLibrary.PrintString` "You collcted a key fragment")
          (`self.K2_DestroyActor`))))))

(event `self.Sphere.OnComponentBeginOverlap`
  (params (OverlappedComponent :type "PrimitiveComponent Object Reference") (OtherActor :type "Actor Object Reference") (OtherComp :type "PrimitiveComponent Object Reference") (OtherBodyIndex :type Integer) (bFromSweep :type Boolean) (SweepResult :type "HitResult Structure (by ref)"))
  (cast `/Game/Blueprints/Characters/0_Base_Human` OtherActor)
  (`self.EnableInput` (`GameplayStatics.GetPlayerController` 0))
  (`KismetSystemLibrary.PrintString` "PICK UP KEY FRAGMENT")
  (goto _label :!via `Open`))

(event `self.Sphere.OnComponentEndOverlap`
  (params (OverlappedComponent :type "PrimitiveComponent Object Reference") (OtherActor :type "Actor Object Reference") (OtherComp :type "PrimitiveComponent Object Reference") (OtherBodyIndex :type Integer))
  (cast `/Game/Blueprints/Characters/0_Base_Human` OtherActor)
  (`self.DisableInput` (`GameplayStatics.GetPlayerController` 0))
  (goto _label :!via `Close`))

(event `Key|Q`
  (params (Key :type "Key Structure"))
  (:`Pressed`
    (goto _label)))

(fn `UserConstructionScript`)