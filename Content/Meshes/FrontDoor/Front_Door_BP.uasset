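; Front door actor that serves as the level's exit check, testing whether all key sections have been found.
; Overlap of InteractionZone by a 0_Base_Human toggles player 0's input and opens or closes a gate.
; E or Q enters that gate, which reads KeySectionsFound from GameplayGM.
; At three sections it prints a game-over transition message as a placeholder, otherwise a missing-key message.
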(event `Key|E`
  (params (Key :type "Key Structure"))
  (:`Pressed`
    (`/Engine/EditorBlueprintResources/StandardMacros.Gate` true :!label _label
      (:`Exit`
        (bind _asgameplay_gm (cast `/Game/Blueprints/Gameplay/GameplayGM` (`GameplayStatics.GetGameMode`)))
        (if (== (`/Game/Blueprints/Gameplay/GameplayGM.KeySectionsFound` _asgameplay_gm) 3)
          (`KismetSystemLibrary.PrintString` "All Keys discovered. >> To Game Over Screen")
          (else
            (`KismetSystemLibrary.PrintString` "Still Missing Key")))))))

(event `self.Interaction Zone.OnComponentBeginOverlap`
  (params (OverlappedComponent :type "PrimitiveComponent Object Reference") (OtherActor :type "Actor Object Reference") (OtherComp :type "PrimitiveComponent Object Reference") (OtherBodyIndex :type Integer) (bFromSweep :type Boolean) (SweepResult :type "HitResult Structure (by ref)"))
  (cast `/Game/Blueprints/Characters/0_Base_Human` OtherActor)
  (`self.EnableInput` (`GameplayStatics.GetPlayerController` 0))
  (goto _label :!via `Open`))

(event `self.Interaction Zone.OnComponentEndOverlap`
  (params (OverlappedComponent :type "PrimitiveComponent Object Reference") (OtherActor :type "Actor Object Reference") (OtherComp :type "PrimitiveComponent Object Reference") (OtherBodyIndex :type Integer))
  (cast `/Game/Blueprints/Characters/0_Base_Human` OtherActor)
  (`self.DisableInput` (`GameplayStatics.GetPlayerController` 0))
  (goto _label :!via `Close`))

(event `Key|Q`
  (params (Key :type "Key Structure"))
  (:`Pressed`
    (goto _label)))

(fn `UserConstructionScript`)