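; Hinged door that players open and close from either side with E or gamepad, and that the Wraith can also operate.
; Front and back triggers open input gates feeding FlipFlops, which play or reverse two timelines that rotate the mesh each way, with sound.
; Per-side access flags fall back to random temporary locked messages.
; Tick optionally auto-closes after a delay, while mesh hits call the Wraith's OpenDoor and force-open events bypass the overlaps.
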(event `self.ReceiveBeginPlay`
  (`ActorComponent.K2_DestroyComponent` (`self.Open1`))
  (`ActorComponent.K2_DestroyComponent` (`self.Open2`)))

(event `Display Message`
  ;[1 1 1] Inaccessible Door Message
  (`|MultiGate` true true (`KismetMathLibrary.RandomInteger` 5)
    (:`Out 0`
      (bind _output_get (set `self.Locked Message 1` "Fawwwk!"))
      ;;[1 0.3545 0] Temp
      (`KismetSystemLibrary.PrintString` (`KismetTextLibrary.Conv_TextToString` _output_get)))
    (:`Out 1`
      (bind _output_get_2 (set `self.Locked Message 2` "Knock Knock"))
      (`KismetSystemLibrary.PrintString` (`KismetTextLibrary.Conv_TextToString` _output_get_2)))
    (:`Out 2`
      (bind _output_get_3 (set `self.Locked Message 3` "I need a pack of C4"))
      (`KismetSystemLibrary.PrintString` (`KismetTextLibrary.Conv_TextToString` _output_get_3)))))

(event `self.ReceiveTick`
  (params (DeltaSeconds :type "Float (single-precision)"))
  (bind _isintriggerzone (`self.isInTriggerZone`))
  (bind _yaw (.yaw (`SceneComponent.RelativeRotation` (`self.StaticMesh`))))
  ;[1 1 1] Close Door Automatically
  (if (`self.DoorClosesAutomatic`)
    (if (`self.IsDoorOpenFront?`)
      (if _isintriggerzone
        (`KismetSystemLibrary.RetriggerableDelay` (`KismetMathLibrary.Conv_IntToDouble` (`self.CloseTime(sec)`)))
        (if (> _yaw 89.0)
          (`self.TriggerFrontCloseDoor`)))
      (elif (`self.IsDoorOpenBack?`)
        (if _isintriggerzone
          (`KismetSystemLibrary.RetriggerableDelay` (`KismetMathLibrary.Conv_IntToDouble` (`self.CloseTime(sec)`)))
          (if (< _yaw -89.0)
            (`self.TriggerBackCloseDoor`)))))))

(event `self.Front Trigger.OnComponentBeginOverlap`
  (params (OverlappedComponent :type "PrimitiveComponent Object Reference") (OtherActor :type "Actor Object Reference") (OtherComp :type "PrimitiveComponent Object Reference") (OtherBodyIndex :type Integer) (bFromSweep :type Boolean) (SweepResult :type "HitResult Structure (by ref)"))
  (bind _staticmesh (`self.StaticMesh`))
  ;[1 1 1] Door Open/Close
  (cast `/Game/Blueprints/Characters/0_Base_Human` OtherActor
    (:`then`
      (set `self.isInTriggerZone` true)
      (`self.EnableInput` (`GameplayStatics.GetPlayerController` 0))
      (goto _label_2 :!via `Open`))
    (:`CastFailed`
      (cast `/Game/Characters/Wraith/Wraith` OtherActor)
      (set `self.LastActivated` true :!label _label)
      (set `self.FrontTrigger` true)
      (set `self.isInTriggerZone` true)
      (goto _label_2 :!via `Open`))))

(event `Key|E`
  (params (Key :type "Key Structure"))
  (bind _staticmesh (`self.StaticMesh`))
  ;[1 1 1] Door Open/Close
  (:`Pressed`
    (`/Engine/EditorBlueprintResources/StandardMacros.Gate` true :!label _label_2
      (:`Exit`
        (if (`self.CanOpenFromFront?`)
          (if (`self.isBackTriggerActive`)
            (set `self.isBackTriggerActive` false :!label _label_3)
            (`/Engine/EditorBlueprintResources/StandardMacros.FlipFlop` :!label _label_4
              (:`A`
                (set `self.isBackTriggerActive` true)
                (set `self.IsDoorOpenBack?` true)
                (bind (_direction _close_transition) (`Timeline|Close Door` :!label _label_5)
                  (:`Update`
                    (`|ExecutionSequence`
                      (:`then_0`
                        (`/Engine/EditorBlueprintResources/StandardMacros.DoOnce` false :!label _label_6
                          (:`Completed`
                            (`GameplayStatics.PlaySoundAtLocation` "/Game/Audio/SFX/DoorClose.DoorClose"))))
                      (:`then_1`
                        (`SceneComponent.K2_SetRelativeRotation` _staticmesh (`KismetMathLibrary.MakeRotator` 0.0 0.0 (* _close_transition (`self.Rotation`))) false false))))
                  (:`Finished`
                    (goto _label_6 :!via `Reset`))))
              (:`B`
                (set `self.isBackTriggerActive` false)
                (set `self.IsDoorOpenBack?` false)
                (goto _label_5 :!via `Reverse`)))
            (else
              (`/Engine/EditorBlueprintResources/StandardMacros.FlipFlop` :!label _label_7
                (:`A`
                  (set `self.isFrontTriggerActive` true)
                  (set `self.IsDoorOpenFront?` true)
                  (bind (_direction_2 _open_transition) (`Timeline|Open Door` :!label _label_8)
                    (:`Update`
                      (`|ExecutionSequence`
                        (:`then_0`
                          (`/Engine/EditorBlueprintResources/StandardMacros.DoOnce` false :!label _label_9
                            (:`Completed`
                              (`GameplayStatics.PlaySoundAtLocation` "/Game/Audio/SFX/DoorOpen.DoorOpen"))))
                        (:`then_1`
                          (`SceneComponent.K2_SetRelativeRotation` _staticmesh (`KismetMathLibrary.MakeRotator` 0.0 0.0 (* _open_transition (`self.Rotation`))) false false))))
                    (:`Finished`
                      (goto _label_9 :!via `Reset`))))
                (:`B`
                  (set `self.isFrontTriggerActive` false)
                  (set `self.IsDoorOpenFront?` false)
                  (goto _label_8 :!via `Reverse`)))))
          (elif (`self.IsDoorOpenBack?`)
            (goto _label_3)
            (else
              (`self.Display Message` :!label _label_10))))))))

(event `ForceOpenFront`
  ;[1 1 1] Door Open/Close
  (`|ExecutionSequence`
    (:`then_0`
      (goto _label))
    (:`then_1`
      (goto _label_2))
    (:`then_2`
      (goto _label_2 :!via `Close`))))

(event `Key|Gamepad_FaceButton_Left`
  (params (Key :type "Key Structure"))
  ;[1 1 1] Door Open/Close
  (:`Pressed`
    (goto _label_2)))

(event `self.Front Trigger.OnComponentEndOverlap`
  (params (OverlappedComponent :type "PrimitiveComponent Object Reference") (OtherActor :type "Actor Object Reference") (OtherComp :type "PrimitiveComponent Object Reference") (OtherBodyIndex :type Integer))
  ;[1 1 1] Door Open/Close
  (cast `/Game/Blueprints/Characters/0_Base_Human` OtherActor
    (:`then`
      (set `self.isInTriggerZone` false)
      (`self.DisableInput` (`GameplayStatics.GetPlayerController` 0))
      (goto _label_2 :!via `Close`))
    (:`CastFailed`
      (cast `/Game/Characters/Wraith/Wraith` OtherActor)
      (set `self.FrontTrigger` false)
      (set `self.isInTriggerZone` false)
      (goto _label_2 :!via `Close`))))

(event `TriggerFrontCloseDoor`
  ;[1 1 1] Door Open/Close
  (goto _label_7))

(event `WraithOpen`
  ;[1 1 1] Door Open/Close
  (if (and (== (`self.BackTrigger`) true) (== (`self.FrontTrigger`) true))
    (if (`self.LastActivated`)
      _
      (else
        (goto _label_2)))
    (else
      (`|ExecutionSequence`
        (:`then_0`
          (goto _label_2))
        (:`then_1`
          _))))
  (`/Engine/EditorBlueprintResources/StandardMacros.Gate` true :!label _label_11
    (:`Exit`
      (if (`self.CanOpenFromBack?`)
        (if (`self.isFrontTriggerActive`)
          _
          (else
            (goto _label_4)))
        (elif (`self.IsDoorOpenFront?`)
          _
          (else
            (goto _label_10))))
      (set `self.isFrontTriggerActive` false)
      (goto _label_7))))

(event `TriggerBackCloseDoor`
  ;[1 1 1] Door Open/Close
  (goto _label_4))

(event `self.Back Trigger.OnComponentBeginOverlap`
  (params (OverlappedComponent :type "PrimitiveComponent Object Reference") (OtherActor :type "Actor Object Reference") (OtherComp :type "PrimitiveComponent Object Reference") (OtherBodyIndex :type Integer) (bFromSweep :type Boolean) (SweepResult :type "HitResult Structure (by ref)"))
  ;[1 1 1] Door Open/Close
  (cast `/Game/Blueprints/Characters/0_Base_Human` OtherActor
    (:`then`
      (set `self.isInTriggerZone` true)
      (`self.EnableInput` (`GameplayStatics.GetPlayerController` 0))
      (goto _label_11 :!via `Open`))
    (:`CastFailed`
      (cast `/Game/Characters/Wraith/Wraith` OtherActor)
      (set `self.LastActivated` false :!label _label_12)
      (set `self.BackTrigger` true)
      (set `self.isInTriggerZone` true)
      (goto _label_11 :!via `Open`))))

(event `Key|E`
  (params (Key :type "Key Structure"))
  ;[1 1 1] Door Open/Close
  (:`Pressed`
    (goto _label_11)))

(event `ForceOpenBack`
  ;[1 1 1] Door Open/Close
  (`|ExecutionSequence`
    (:`then_0`
      (goto _label_12))
    (:`then_1`
      (goto _label_11))
    (:`then_2`
      (goto _label_11 :!via `Close`))))

(event `Key|Gamepad_FaceButton_Left`
  (params (Key :type "Key Structure"))
  ;[1 1 1] Door Open/Close
  (:`Pressed`
    (goto _label_11)))

(event `self.Back Trigger.OnComponentEndOverlap`
  (params (OverlappedComponent :type "PrimitiveComponent Object Reference") (OtherActor :type "Actor Object Reference") (OtherComp :type "PrimitiveComponent Object Reference") (OtherBodyIndex :type Integer))
  ;[1 1 1] Door Open/Close
  (cast `/Game/Blueprints/Characters/0_Base_Human` OtherActor
    (:`then`
      (set `self.isInTriggerZone` false)
      (`self.DisableInput` (`GameplayStatics.GetPlayerController` 0))
      (goto _label_11 :!via `Close`))
    (:`CastFailed`
      (cast `/Game/Characters/Wraith/Wraith` OtherActor)
      (set `self.BackTrigger` false)
      (set `self.isInTriggerZone` false)
      (goto _label_11 :!via `Close`))))

(event `self.StaticMesh.OnComponentHit`
  (params (HitComponent :type "PrimitiveComponent Object Reference") (OtherActor :type "Actor Object Reference") (OtherComp :type "PrimitiveComponent Object Reference") (NormalImpulse :type "Vector Structure") (Hit :type "HitResult Structure (by ref)"))
  (bind _aswraith (cast `/Game/Characters/Wraith/Wraith` OtherActor))
  (`|ExecutionSequence`
    (:`then_0`
      (`/Game/Characters/Wraith/Wraith.OpenDoor` _aswraith self))))

(fn `UserConstructionScript`)