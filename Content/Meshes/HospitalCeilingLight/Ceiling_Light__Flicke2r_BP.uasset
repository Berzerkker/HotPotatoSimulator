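; A hospital ceiling light Blueprint that flickers on and off at random intervals.
; Tick feeds a Delay of up to one second, then a FlipFlop alternates between the lit and unlit states.
; Each state swaps the static mesh between emissive and non-emissive materials and sets the spotlight intensity to match, so fixture glow and cast light switch together.
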(event `self.ReceiveTick`
  (params (DeltaSeconds :type "Float (single-precision)"))
  (`KismetSystemLibrary.Delay` (`KismetMathLibrary.RandomFloatInRange` 0.0 1.0))
  (`/Engine/EditorBlueprintResources/StandardMacros.FlipFlop`
    (:`A`
      (`|ExecutionSequence`
        (:`then_0`
          (`PrimitiveComponent.SetMaterial` (`self.StaticMesh`) 0 "/Game/Meshes/HospitalCeilingLight/CelingLight_Emissive_Mat.CelingLight_Emissive_Mat"))
        (:`then_1`
          (`LightComponent.SetIntensity` (`self.SpotLight`) 2000.0))))
    (:`B`
      (`|ExecutionSequence`
        (:`then_0`
          (`PrimitiveComponent.SetMaterial` (`self.StaticMesh`) 0 "/Game/Meshes/HospitalCeilingLight/CelingLight_NonEmissive_Mat.CelingLight_NonEmissive_Mat"))
        (:`then_1`
          (`LightComponent.SetIntensity` (`self.SpotLight`) 0.0))))))

(fn `UserConstructionScript`)