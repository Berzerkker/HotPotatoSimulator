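; Hospital ceiling light Blueprint that flickers while a threat (Giant) is within its detection sphere.
; Sphere begin and end overlaps share a FlipFlop that toggles the in-range flag, restoring the lit state when cleared.
; While flagged, Tick alternates emissive material and spotlight intensity after a Delay scaled from the summed X/Y offset to GameplayGM's WraithLocation, obtained via a line trace, so flicker generally quickens with proximity.
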(event `self.ReceiveBeginPlay`
  (`SphereComponent.SetSphereRadius` (`self.Detection Range`) (`self.Threat Detection Radius`) true))

(event `self.Detection Range.OnComponentBeginOverlap`
  (params (OverlappedComponent :type "PrimitiveComponent Object Reference") (OtherActor :type "Actor Object Reference") (OtherComp :type "PrimitiveComponent Object Reference") (OtherBodyIndex :type Integer) (bFromSweep :type Boolean) (SweepResult :type "HitResult Structure (by ref)"))
  (cast `/Game/Blueprints/Characters/Giant` OtherActor)
  (`/Engine/EditorBlueprintResources/StandardMacros.FlipFlop` :!label _label
    (:`A`
      (set `self.isThreatInRange` true))
    (:`B`
      (set `self.isThreatInRange` false)
      (`|ExecutionSequence`
        (:`then_0`
          (`PrimitiveComponent.SetMaterial` (`self.StaticMesh`) 0 "/Game/Meshes/HospitalCeilingLight/CelingLight_Emissive_Mat.CelingLight_Emissive_Mat"))
        (:`then_1`
          (`LightComponent.SetIntensity` (`self.SpotLight`) 2000.0))))))

(event `self.Detection Range.OnComponentEndOverlap`
  (params (OverlappedComponent :type "PrimitiveComponent Object Reference") (OtherActor :type "Actor Object Reference") (OtherComp :type "PrimitiveComponent Object Reference") (OtherBodyIndex :type Integer))
  (cast `/Game/Blueprints/Characters/Giant` OtherActor)
  (goto _label))

(event `self.ReceiveTick`
  (params (DeltaSeconds :type "Float (single-precision)"))
  (if (`self.isThreatInRange`)
    (bind _asgameplay_gm (cast `/Game/Blueprints/Gameplay/GameplayGM` (`GameplayStatics.GetGameMode`)))
    (bind _outhit (`KismetSystemLibrary.LineTraceSingle` (`SceneComponent.K2_GetComponentLocation` (`self.StaticMesh`)) (`/Game/Blueprints/Gameplay/GameplayGM.Wraith Location` _asgameplay_gm) "TraceTypeQuery1" true))
    (bind (_bblockinghit _binitialoverlap _time _distance _location _impactpoint _normal _impactnormal _physmat _hitactor _hitcomponent _hitbonename _hititem _faceindex _tracestart _traceend) (`GameplayStatics.BreakHitResult` _outhit))
    (`KismetSystemLibrary.Delay` (`KismetMathLibrary.Abs` (/ (+ (.x (- _tracestart _traceend)) (.y (- _tracestart _traceend))) 1000.0)))
    (`/Engine/EditorBlueprintResources/StandardMacros.FlipFlop`
      (:`A`
        (`|ExecutionSequence`
          (:`then_0`
            (`PrimitiveComponent.SetMaterial` (`self.StaticMesh`) 0 "/Game/Meshes/HospitalCeilingLight/CelingLight_Emissive_Mat.CelingLight_Emissive_Mat"))
          (:`then_1`
            (`LightComponent.SetIntensity` (`self.SpotLight`) 2000.0))))
      (:`B`
        (`|ExecutionSequence`
          (:`then_0`
            (`PrimitiveComponent.SetMaterial` (`self.StaticMesh`) 0 "/Game/Meshes/HospitalCeilingLight/CelingLight_NonEmissive_Mat.CelingLight_NonEmissive_Mat"))
          (:`then_1`
            (`LightComponent.SetIntensity` (`self.SpotLight`) 0.0)))))))

(fn `UserConstructionScript`)