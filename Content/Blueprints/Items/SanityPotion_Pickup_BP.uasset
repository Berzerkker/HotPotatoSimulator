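; Sanity potion pickup that players grab with E inside its detection zone, adjusting their sanity before destroying itself.
; If the first Wraith found is within range on pickup, it teleports to a random navmesh point around the player, chosen by path length between min and max, then wanders.
; A delayed Tick replays a timeline that pulses material glow, creating a dynamic instance on each update.
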(event `Key|E`
  (params (Key :type "Key Structure"))
  (:`Pressed`
    (`/Engine/EditorBlueprintResources/StandardMacros.Gate` true :!label _label
      (:`Exit`
        (bind _ashuman (cast `/Game/Blueprints/Characters/Human` (`GameplayStatics.GetPlayerCharacter` 0)))
        (set `self.PlayerObject` _ashuman)
        (`/Game/Blueprints/Characters/0_Base_Human.UpdateSanity` (`self.PlayerObject`) (`self.Amount`))
        (bind _outactors (`GameplayStatics.GetAllActorsOfClass` "/Game/Blueprints/Characters/Wraith.Wraith_C"))
        (bind _output_get (set `self.WraithObject` (`|GetArrayItem` _outactors)))
        (if (< (`KismetMathLibrary.VSize` (- (`SceneComponent.K2_GetComponentLocation` (`Character.CapsuleComponent` _output_get)) (`SceneComponent.K2_GetComponentLocation` (`Character.CapsuleComponent` (`self.PlayerObject`))))) (`self.TeleportWraithDistance`))
          (`self.TeleportWraith`))
        (`self.K2_DestroyActor`)))))

(event `self.DetectionZone.OnComponentBeginOverlap`
  (params (OverlappedComponent :type "PrimitiveComponent Object Reference") (OtherActor :type "Actor Object Reference") (OtherComp :type "PrimitiveComponent Object Reference") (OtherBodyIndex :type Integer) (bFromSweep :type Boolean) (SweepResult :type "HitResult Structure (by ref)"))
  (cast `/Game/Blueprints/Characters/0_Base_Human` OtherActor)
  (`self.EnableInput` (`GameplayStatics.GetPlayerController` 0))
  (`KismetSystemLibrary.PrintString` "Press E to pick up potion")
  (goto _label :!via `Open`))

(event `Key|Q`
  (params (Key :type "Key Structure"))
  (:`Pressed`
    (goto _label :!via `Close`)))

(event `self.DetectionZone.OnComponentEndOverlap`
  (params (OverlappedComponent :type "PrimitiveComponent Object Reference") (OtherActor :type "Actor Object Reference") (OtherComp :type "PrimitiveComponent Object Reference") (OtherBodyIndex :type Integer))
  (cast `/Game/Blueprints/Characters/0_Base_Human` OtherActor)
  (`self.DisableInput` (`GameplayStatics.GetPlayerController` 0)))

(event `self.ReceiveTick`
  (params (DeltaSeconds :type "Float (single-precision)"))
  (`KismetSystemLibrary.Delay` 5.0)
  (bind (_direction _newtrack_0) (`Timeline|Timeline_0` :!via `PlayFromStart`)
    (:`Update`
      (bind _returnvalue (`PrimitiveComponent.CreateDynamicMaterialInstance` (`self.StaticMesh`) 0 "/Game/Meshes/SanityPotionPickup/SanityPotion_Pickup_Mat_Inst.SanityPotion_Pickup_Mat_Inst"))
      (`MaterialInstanceDynamic.SetScalarParameterValue` _returnvalue "GlowIntensity" _newtrack_0))))

(fn `TeleportWraith`
  (bind _playerlocation (`self.PlayerLocation`))
  (bind _wraithobject (`self.WraithObject`))
  (bind _wraithobject_2 (`self.WraithObject`))
  (bind (_teleportpoint_x _teleportpoint_y) (`KismetMathLibrary.BreakVector` (`self.TeleportPoint`)))
  (set `self.PlayerLocation` (`self.K2_GetActorLocation` (`self.PlayerObject`)))
  (while (`self.BadDistance`)
    (bind _output_get (set `self.TeleportPoint` (`NavigationSystem.K2_GetRandomLocationInNavigableRadius` _playerlocation 2000.0)))
    (bind _returnvalue (`NavigationSystem.FindPathToLocationSynchronously` _playerlocation _output_get (`self.WraithObject`)))
    (bind _returnvalue_2 (`NavigationPath.GetPathLength` _returnvalue))
    (if (and (> (`self.TeleportWraithMax`) _returnvalue_2) (> _returnvalue_2 (`self.TeleportWraithMin`)))
      (set `self.BadDistance` false)
      (set `self.TeleportPoint` (`KismetMathLibrary.MakeVector` _teleportpoint_x _teleportpoint_y 100.0))))
  (bind _returnvalue_3 (`self.K2_TeleportTo` _wraithobject_2 (`self.TeleportPoint`) (`self.K2_GetActorRotation` _wraithobject_2)))
  (if _returnvalue_3
    ;[1 1 1] Set to wander unless raging
    (switch `int` (`/Game/Blueprints/Characters/Wraith.Mode` _wraithobject)
      (:`Default`
        _)
      (:`0`
        _)
      (:`1`
        _)
      (:`2`
        _))
    (`/Game/Blueprints/Characters/Wraith.Wander` _wraithobject)
    (else
      (`KismetSystemLibrary.PrintString` "Failed Teleport")
      (`self.TeleportWraith`))))

(fn `UserConstructionScript`)