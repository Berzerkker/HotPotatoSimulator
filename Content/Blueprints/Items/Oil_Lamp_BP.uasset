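; Oil lamp item that acts as a key fragment detector, shifting its light from warm toward blue as a fragment gets closer.
; Sphere overlap stores the fragment and sets KeyDetected on GameplayGM.
; While that is set, Tick traces to the fragment and uses distance to drive light color and FlameIntensity, creating a dynamic material each frame.
; When it clears, a DoOnce restores defaults; DetectionZone prints a pickup prompt for humans.
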(event `self.ReceiveBeginPlay`
  ;[1 1 1] Create GameMode Variable
  (bind _asgameplay_gm (cast `/Game/Blueprints/Gameplay/GameplayGM` (`GameplayStatics.GetGameMode`)))
  (set `self.GameplayGameMode` _asgameplay_gm))

(event `self.ReceiveTick`
  (params (DeltaSeconds :type "Float (single-precision)"))
  ;[1 0 0] Tick Chain
  (`self.GetDistanceSetLightColor`))

(event `self.Sphere.OnComponentBeginOverlap`
  (params (OverlappedComponent :type "PrimitiveComponent Object Reference") (OtherActor :type "Actor Object Reference") (OtherComp :type "PrimitiveComponent Object Reference") (OtherBodyIndex :type Integer) (bFromSweep :type Boolean) (SweepResult :type "HitResult Structure (by ref)"))
  ;[1 1 1] Change Light Color if Key is Nearby
  ;;[1 1 1] Detect Key Fragment Location
  (bind _askey_fragment_1 (cast `/Game/Blueprints/Keys/KeyFragment1` OtherActor)
    (:`then`
      (set `self.NearbyKeyFragment` _askey_fragment_1))
    (:`CastFailed`
      (bind _askey_fragment_2 (cast `/Game/Blueprints/Keys/KeyFragment2` OtherActor)
        (:`then`
          (set `self.NearbyKeyFragment` _askey_fragment_2))
        (:`CastFailed`
          (bind _askey_fragment_3 (cast `/Game/Blueprints/Keys/KeyFragment3` OtherActor))
          (set `self.NearbyKeyFragment` _askey_fragment_3)))))
  (set `/Game/Blueprints/Gameplay/GameplayGM.KeyDetected` true (`self.GameplayGameMode`))
  (goto _label :!via `Reset`))

(event `GetDistanceSetLightColor`
  ;[1 1 1] Change Light Color if Key is Nearby
  ;;[1 1 1] Draw Trace to Key and Change Light Color Accordingly
  ;;;[1 1 1] Get Distance Between Lamp and Key Fragment
  (if (`/Game/Blueprints/Gameplay/GameplayGM.KeyDetected` (`self.GameplayGameMode`))
    (bind _outhit (`KismetSystemLibrary.LineTraceSingle` (`SceneComponent.K2_GetComponentLocation` (`self.StaticMesh`)) (`self.K2_GetActorLocation` (`self.NearbyKeyFragment`)) "TraceTypeQuery1"))
    (bind (_bblockinghit _binitialoverlap _time _distance _location _impactpoint _normal _impactnormal _physmat _hitactor _hitcomponent _hitbonename _hititem _faceindex _tracestart _traceend) (`GameplayStatics.BreakHitResult` _outhit))
    (bind _returnvalue (/ (`KismetMathLibrary.GetPointDistanceToLine` _tracestart _traceend) 1000.0))
    ;;;[1 1 1] Pan Light and Flame Color
    (`LightComponent.SetLightColor` (`self.PointLight`) (`KismetMathLibrary.LinearColorLerp` (struct :`G` 0.574001 :`B` 1.0 :`A` 1.0) (struct :`R` 1.0 :`G` 0.887923 :`B` 0.768151 :`A` 1.0) _returnvalue) true)
    (bind _returnvalue_2 (`PrimitiveComponent.CreateDynamicMaterialInstance` (`self.StaticMesh`) 0 "/Game/Meshes/OilLamp/OilLamp_Mat_Inst.OilLamp_Mat_Inst"))
    (bind _returnvalue_3 (`KismetMathLibrary.InverseLerp` 2.0 0.0 _returnvalue))
    (if (not (< _returnvalue_3 0.2))
      (`MaterialInstanceDynamic.SetScalarParameterValue` _returnvalue_2 "FlameIntensity" _returnvalue_3))
    (else
      ;;;[1 1 1] Change To Default Light Settings after Key Fragment is picked up
      (`/Engine/EditorBlueprintResources/StandardMacros.DoOnce` false :!label _label
        (:`Completed`
          (`LightComponent.SetLightColor` (`self.PointLight`) (struct :`R` 1.0 :`G` 0.887923 :`B` 0.768151 :`A` 1.0) true)
          (bind _returnvalue_4 (`PrimitiveComponent.CreateDynamicMaterialInstance` (`self.StaticMesh`) 0 "/Game/Meshes/OilLamp/OilLamp_Mat_Inst.OilLamp_Mat_Inst"))
          (`MaterialInstanceDynamic.SetScalarParameterValue` _returnvalue_4 "FlameIntensity" 0.2))))))

(event `self.DetectionZone.OnComponentBeginOverlap`
  (params (OverlappedComponent :type "PrimitiveComponent Object Reference") (OtherActor :type "Actor Object Reference") (OtherComp :type "PrimitiveComponent Object Reference") (OtherBodyIndex :type Integer) (bFromSweep :type Boolean) (SweepResult :type "HitResult Structure (by ref)"))
  ;[1 1 1] Show Pick Up Lamp Indicator
  (cast `/Game/Blueprints/Characters/0_Base_Human` OtherActor)
  (`KismetSystemLibrary.PrintString` "Pick Up Lamp"))

(fn `UserConstructionScript`)