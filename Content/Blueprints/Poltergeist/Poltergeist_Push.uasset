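; Poltergeist push trap that fires a single radial force burst when a human enters its trigger sphere.
; A sphere overlap filtered to the base human class passes through a DoOnce, so only the first such entry triggers it.
; It copies the actor's impulse and force strength variables onto the RadialForce component, activates it, then deactivates it after a short delay.
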(event `self.Sphere.OnComponentBeginOverlap`
  (params (OverlappedComponent :type "PrimitiveComponent Object Reference") (OtherActor :type "Actor Object Reference") (OtherComp :type "PrimitiveComponent Object Reference") (OtherBodyIndex :type Integer) (bFromSweep :type Boolean) (SweepResult :type "HitResult Structure (by ref)"))
  (bind _radialforce (`self.RadialForce`))
  ;[1 1 1] Effect Chain
  (cast `/Game/Blueprints/Characters/0_Base_Human` OtherActor)
  (`/Engine/EditorBlueprintResources/StandardMacros.DoOnce` false
    (:`Completed`
      (set `RadialForceComponent.ImpulseStrength` (`self.ImpulseStrength`) _radialforce)
      (set `RadialForceComponent.ForceStrength` (`self.ForceStrength`) _radialforce)
      (`ActorComponent.Activate` _radialforce false)
      (`KismetSystemLibrary.Delay` 0.5)
      (`ActorComponent.Deactivate` (`self.RadialForce`)))))

(fn `UserConstructionScript`)