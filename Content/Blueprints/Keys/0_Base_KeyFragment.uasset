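; Base key fragment pickup that a human player collects with E or Q while inside its sphere, using overlap-driven input and a Gate.
; Collection runs once, raising the GameplayGM fragment count, notifying the first Wraith, clearing key detection, redrawing the path and destroying the actor.
; A Tick-driven delay replays a timeline that pulses the mesh's glow, creating a dynamic material instance on each update.
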(event `Key|E`
  (params (Key :type "Key Structure"))
  (:`Pressed`
    (`/Engine/EditorBlueprintResources/StandardMacros.Gate` true :!label _label
      (:`Exit`
        (`/Engine/EditorBlueprintResources/StandardMacros.DoOnce` false
          (:`Completed`
            (bind _asgameplay_gm (cast `/Game/Blueprints/Gameplay/GameplayGM` (`GameplayStatics.GetGameMode`)))
            (bind _output_get (set `/Game/Blueprints/Gameplay/GameplayGM.KeySectionsFound` (+ (`/Game/Blueprints/Gameplay/GameplayGM.KeySectionsFound` _asgameplay_gm) 1) _asgameplay_gm))
            (bind _outactors (`GameplayStatics.GetAllActorsOfClass` "/Game/Blueprints/Characters/Wraith.Wraith_C"))
            (`/Game/Blueprints/Characters/Wraith.KeySectionFound` (`|GetArrayItem` _outactors) _output_get)
            (`KismetSystemLibrary.PrintString` "You collcted a key fragment")
            (set `/Game/Blueprints/Gameplay/GameplayGM.KeyDetected` false _asgameplay_gm)
            (`/Game/Blueprints/Gameplay/GameplayGM.DrawPath` _asgameplay_gm)
            (`self.K2_DestroyActor`)))))))

(event `self.Sphere.OnComponentBeginOverlap`
  (params (OverlappedComponent :type "PrimitiveComponent Object Reference") (OtherActor :type "Actor Object Reference") (OtherComp :type "PrimitiveComponent Object Reference") (OtherBodyIndex :type Integer) (bFromSweep :type Boolean) (SweepResult :type "HitResult Structure (by ref)"))
  (cast `/Game/Blueprints/Characters/0_Base_Human` OtherActor)
  (`self.EnableInput` (`GameplayStatics.GetPlayerController` 0))
  (`KismetSystemLibrary.PrintString` "PICK UP KEY FRAGMENT")
  (goto _label :!via `Open`))

(event `self.Sphere.OnComponentEndOverlap`
  (params (OverlappedComponent :type "PrimitiveComponent Object Reference") (OtherActor :type "Actor Object Reference") (OtherComp :type "PrimitiveComponent Object Reference") (OtherBodyIndex :type Integer))
  (cast `/Game/Blueprints/Characters/0_Base_Human` OtherActor)
  (`self.DisableInput` (`GameplayStatics.GetPlayerController` 0))
  (goto _label :!via `Close`))

(event `Key|Q`
  (params (Key :type "Key Structure"))
  (:`Pressed`
    (goto _label)))

(event `self.ReceiveTick`
  (params (DeltaSeconds :type "Float (single-precision)"))
  ;[1 1 1] Glow Identifier
  (`KismetSystemLibrary.Delay` 5.0)
  (bind (_direction _newtrack_0) (`Timeline|Timeline_0` :!via `PlayFromStart`)
    (:`Update`
      (bind _returnvalue (`PrimitiveComponent.CreateDynamicMaterialInstance` (`self.Fragmented_Key_Exit_Key_Fragment`) 0 "/Game/Meshes/FragmentedExitKey/KeyFragment_Mat_Inst.KeyFragment_Mat_Inst"))
      (`MaterialInstanceDynamic.SetScalarParameterValue` _returnvalue "GlowIntensity" _newtrack_0))))

(fn `UserConstructionScript`)