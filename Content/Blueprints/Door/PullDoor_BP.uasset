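; PullDoor_BP is a hinged door that swings open automatically when characters approach from either side.
; Inside and outside triggers set swing direction, with speed scaled to a human's walk or run speed; only outside opening disables door collision.
; Leaving the close trigger starts closing and restores collision, unless that human's Enemy still overlaps the door.
; Tick rotates the hinge incrementally, snapping it at ninety degrees or closed within a tolerance.
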(event `self.Close Collision.OnComponentEndOverlap`
  (params (OverlappedComponent :type "PrimitiveComponent Object Reference") (OtherActor :type "Actor Object Reference") (OtherComp :type "PrimitiveComponent Object Reference") (OtherBodyIndex :type Integer))
  ;[1 1 1] Close Command
  (bind _ascharacter (cast `Character` OtherActor))
  (bind _as0_base_human (cast `/Game/Blueprints/Characters/0_Base_Human` _ascharacter)
    (:`then`
      (if (not (`self.IsOverlappingActor` (`/Game/Blueprints/Characters/0_Base_Human.Enemy` _as0_base_human)))
        (set `self.Using Door` false :!label _label)
        (set `self.Speed` 200.0)
        (`PrimitiveComponent.SetCollisionEnabled` (`self.Door`) "QueryAndPhysics")))
    (:`CastFailed`
      (goto _label))))

(event `self.Open Collision Out.OnComponentBeginOverlap`
  (params (OverlappedComponent :type "PrimitiveComponent Object Reference") (OtherActor :type "Actor Object Reference") (OtherComp :type "PrimitiveComponent Object Reference") (OtherBodyIndex :type Integer) (bFromSweep :type Boolean) (SweepResult :type "HitResult Structure (by ref)"))
  ;[1 1 1] Open from the Outside Command
  (if (not (`self.Using Door`))
    (cast `Character` OtherActor)
    (bind _as0_base_human (cast `/Game/Blueprints/Characters/0_Base_Human` OtherActor)
      (:`then`
        (bind _running_speed (`/Game/Blueprints/Characters/0_Base_Human.Running Speed` _as0_base_human))
        (if (== (`CharacterMovementComponent.MaxWalkSpeed` (`Character.CharacterMovement` _as0_base_human)) _running_speed)
          (set `self.Speed` (/ _running_speed 2.0))
          (else
            (set `self.Speed` (/ (`/Game/Blueprints/Characters/0_Base_Human.Walking Speed` _as0_base_human) 2.0)))))
      (:`CastFailed`
        _))
    (set `self.Using Door` true)
    (set `self.Direction` (`self.Open Collision Out`))
    (set `self.Direction Value` 1.0)
    (`PrimitiveComponent.SetCollisionEnabled` (`self.Door`) "NoCollision")))

(event `self.Open Collision In.OnComponentBeginOverlap`
  (params (OverlappedComponent :type "PrimitiveComponent Object Reference") (OtherActor :type "Actor Object Reference") (OtherComp :type "PrimitiveComponent Object Reference") (OtherBodyIndex :type Integer) (bFromSweep :type Boolean) (SweepResult :type "HitResult Structure (by ref)"))
  ;[1 1 1] Open from the Inside Command
  (if (not (`self.Using Door`))
    (cast `Character` OtherActor)
    (bind _as0_base_human (cast `/Game/Blueprints/Characters/0_Base_Human` OtherActor)
      (:`then`
        (bind _running_speed (`/Game/Blueprints/Characters/0_Base_Human.Running Speed` _as0_base_human))
        (if (== (`CharacterMovementComponent.MaxWalkSpeed` (`Character.CharacterMovement` _as0_base_human)) _running_speed)
          (set `self.Speed` (/ _running_speed 2.0))
          (else
            (set `self.Speed` (/ (`/Game/Blueprints/Characters/0_Base_Human.Walking Speed` _as0_base_human) 2.0)))))
      (:`CastFailed`
        _))
    (set `self.Using Door` true)
    (set `self.Direction` (`self.Open Collision In`))
    (set `self.Direction Value` -1.0)))

(event `self.ReceiveTick`
  (params (DeltaSeconds :type "Float (single-precision)"))
  (bind _hinge (`self.Hinge`))
  (bind _hinge_2 (`self.Hinge`))
  (bind _hinge_3 (`self.Hinge`))
  (bind _speed (`self.Speed`))
  (bind _ds (`self.DS`))
  ;[1 1 1] Rotation Event
  (set `self.DS` DeltaSeconds)
  (if (`self.Using Door`)
    (if (not (`KismetMathLibrary.NearlyEqual_FloatFloat` (.yaw (.rotation (`SceneComponent.GetRelativeTransform` (`self.Hinge`)))) (* (`self.Direction Value`) 90.0) 5.0))
      (`KismetSystemLibrary.Delay` 0.01)
      (if (== (`self.Direction`) (`self.Open Collision Out`))
        (`SceneComponent.K2_AddRelativeRotation` _hinge (`KismetMathLibrary.MakeRotator` 0.0 0.0 (* (`self.Speed`) (`self.DS`))) false false)
        (else
          (`SceneComponent.K2_AddRelativeRotation` _hinge (`KismetMathLibrary.MakeRotator` 0.0 0.0 (* (`self.Speed`) (`self.DS`) -1.0)) false false)))
      (else
        (`SceneComponent.K2_SetRelativeRotation` _hinge (`KismetMathLibrary.MakeRotator` 0.0 0.0 (* (`self.Direction Value`) 90.0)) false false)
        (goto _label_2 :!via `Reset`)))
    (elif (`KismetMathLibrary.NearlyEqual_FloatFloat` (.yaw (.rotation (`SceneComponent.GetRelativeTransform` _hinge_2))) 0.0 5.0)
      (`/Engine/EditorBlueprintResources/StandardMacros.DoOnce` false :!label _label_2
        (:`Completed`
          (`SceneComponent.K2_SetRelativeRotation` :`self` _hinge_2)))
      (else
        (`KismetSystemLibrary.Delay` 0.01)
        (if (== (`self.Direction`) (`self.Open Collision Out`))
          (`SceneComponent.K2_AddRelativeRotation` _hinge_3 (`KismetMathLibrary.MakeRotator` 0.0 0.0 (* _speed _ds -1.0)) false false)
          (else
            (`SceneComponent.K2_AddRelativeRotation` _hinge_3 (`KismetMathLibrary.MakeRotator` 0.0 0.0 (* _speed _ds)) false false)))))))

(fn `UserConstructionScript`)