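; Interactive double morgue door that a human character opens and closes with E or gamepad left face button.
; The trigger box enables input and gates presses, which either print a random placeholder locked message or FlipFlop two timelines rotating both leaves.
; Optional auto-close retriggers a delay on Tick while the door is open and occupied, then toggles the same FlipFlop once retriggering stops and the delay expires.
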(event `Display Message`
  ;[1 1 1] Inaccessible Door Message
  (`|MultiGate` true true (`KismetMathLibrary.RandomInteger` 5)
    (:`Out 0`
      (bind _output_get (set `self.LockedMessage1` "Fawwwk!"))
      ;;[1 0.3545 0] Temp
      (`KismetSystemLibrary.PrintString` (`KismetTextLibrary.Conv_TextToString` _output_get)))
    (:`Out 1`
      (bind _output_get_2 (set `self.LockedMessage2` ""))
      (`KismetSystemLibrary.PrintString` (`KismetTextLibrary.Conv_TextToString` _output_get_2)))
    (:`Out 2`
      (bind _output_get_3 (set `self.LockedMessage3` ""))
      (`KismetSystemLibrary.PrintString` (`KismetTextLibrary.Conv_TextToString` _output_get_3)))))

(event `self.ReceiveTick`
  (params (DeltaSeconds :type "Float (single-precision)"))
  ;[1 1 1] Close Door Automatically
  (if (`self.DoorClosesAutomatic`)
    (if (`self.isDoorOpenFront`)
      (if (`self.isInTriggerZone`)
        (`KismetSystemLibrary.RetriggerableDelay` (`KismetMathLibrary.Conv_IntToDouble` (`self.CloseTime(sec)`)))
        (`self.TriggerFrontCloseDoor`)))))

(event `self.Door Trigger.OnComponentBeginOverlap`
  (params (OverlappedComponent :type "PrimitiveComponent Object Reference") (OtherActor :type "Actor Object Reference") (OtherComp :type "PrimitiveComponent Object Reference") (OtherBodyIndex :type Integer) (bFromSweep :type Boolean) (SweepResult :type "HitResult Structure (by ref)"))
  ;[1 1 1] Door Open/Close
  (cast `/Game/Blueprints/Characters/0_Base_Human` OtherActor)
  (set `self.isInTriggerZone` true)
  (`self.EnableInput` (`GameplayStatics.GetPlayerController` 0))
  (goto _label :!via `Open`))

(event `Key|E`
  (params (Key :type "Key Structure"))
  ;[1 1 1] Door Open/Close
  (:`Pressed`
    (`/Engine/EditorBlueprintResources/StandardMacros.Gate` true :!label _label
      (:`Exit`
        (if (`self.isLocked`)
          (`self.Display Message`)
          (else
            (`/Engine/EditorBlueprintResources/StandardMacros.FlipFlop` :!label _label_2
              (:`A`
                (set `self.isFrontTriggerActive` true)
                (set `self.isDoorOpenFront` true)
                (`|ExecutionSequence`
                  (:`then_0`
                    ;[1 1 1] Animate Doors
                    (bind (_direction _open_transition) (`Timeline|RightDroorAnimation` :!label _label_3)
                      (:`Update`
                        (`SceneComponent.K2_SetRelativeRotation` (`self.Left_Morgue_Door`) (`KismetMathLibrary.MakeRotator` 0.0 0.0 (* _open_transition (`self.Rotation`))) false false))))
                  (:`then_1`
                    (bind (_direction_2 _open_transition_2) (`Timeline|LeftDoorAnimation` :!label _label_4)
                      (:`Update`
                        (`SceneComponent.K2_SetRelativeRotation` (`self.Right_Morgue_Door`) (`KismetMathLibrary.MakeRotator` 0.0 0.0 (* _open_transition_2 (`self.Rotation`))) false false))))))
              (:`B`
                (set `self.isFrontTriggerActive` false)
                (set `self.isDoorOpenFront` false)
                (`|ExecutionSequence`
                  (:`then_0`
                    (goto _label_3 :!via `Reverse`))
                  (:`then_1`
                    (goto _label_4 :!via `Reverse`)))))))))))

(event `TriggerFrontCloseDoor`
  ;[1 1 1] Door Open/Close
  (goto _label_2))

(event `Key|Gamepad_FaceButton_Left`
  (params (Key :type "Key Structure"))
  ;[1 1 1] Door Open/Close
  (:`Pressed`
    (goto _label)))

(event `self.Door Trigger.OnComponentEndOverlap`
  (params (OverlappedComponent :type "PrimitiveComponent Object Reference") (OtherActor :type "Actor Object Reference") (OtherComp :type "PrimitiveComponent Object Reference") (OtherBodyIndex :type Integer))
  ;[1 1 1] Door Open/Close
  (cast `/Game/Blueprints/Characters/0_Base_Human` OtherActor)
  (set `self.isInTriggerZone` false)
  (`self.DisableInput` (`GameplayStatics.GetPlayerController` 0))
  (goto _label :!via `Close`))

(fn `UserConstructionScript`)