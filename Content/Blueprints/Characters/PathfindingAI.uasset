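; PathfindingAI is a character Blueprint that prototypes path visualization, but its logic is disconnected, so BeginPlay and the construction script do nothing.
; The orphaned graph finds a synchronous navigation path from its location to the first PlayerStart.
; It loops through the path points, chaining long-lived red debug lines through the AILocation variable and spawning a concrete-material decal at each point.
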(event `self.ReceiveBeginPlay`)

(fn `UserConstructionScript`)