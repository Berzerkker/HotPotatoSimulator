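; Giant1 is a giant AI character that pursues the player and shakes the camera with its footfalls.
; While ActivateTheGiant is set, each Tick re-issues a simple move toward the player's 0_Base_Human pawn, then writes the capsule's location to GameplayGM's WraithLocation as a position tracker.
; Overlaps on either foot contact point play a LargeFootsteps world camera shake centred on the mesh, independent of the activation flag.
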(event `self.ReceiveTick`
  (params (DeltaSeconds :type "Float (single-precision)"))
  (if (`self.Activate The Giant`)
    (`|ExecutionSequence`
      (:`then_0`
        (bind _as0_base_human (cast `/Game/Blueprints/Characters/0_Base_Human` (`GameplayStatics.GetPlayerPawn` 0)))
        (`NavigationSystem.SimpleMoveToActor` (`self.GetController`) _as0_base_human))
      (:`then_1`
        ;[1 1 1] GPS
        (bind _asgameplay_gm (cast `/Game/Blueprints/Gameplay/GameplayGM` (`GameplayStatics.GetGameMode`)))
        (set `/Game/Blueprints/Gameplay/GameplayGM.Wraith Location` (`SceneComponent.K2_GetComponentLocation` (`self.CapsuleComponent`)) _asgameplay_gm)))))

(event `self.RT Foot Contact Point.OnComponentBeginOverlap`
  (params (OverlappedComponent :type "PrimitiveComponent Object Reference") (OtherActor :type "Actor Object Reference") (OtherComp :type "PrimitiveComponent Object Reference") (OtherBodyIndex :type Integer) (bFromSweep :type Boolean) (SweepResult :type "HitResult Structure (by ref)"))
  (`GameplayStatics.PlayWorldCameraShake` "/Game/Effects/CameraShakes/LargeFootsteps.LargeFootsteps_C" (`SceneComponent.K2_GetComponentLocation` (`self.Mesh`)) 100.0 1000.0 :!label _label))

(event `self.LF Foot Contact Point.OnComponentBeginOverlap`
  (params (OverlappedComponent :type "PrimitiveComponent Object Reference") (OtherActor :type "Actor Object Reference") (OtherComp :type "PrimitiveComponent Object Reference") (OtherBodyIndex :type Integer) (bFromSweep :type Boolean) (SweepResult :type "HitResult Structure (by ref)"))
  (goto _label))

(fn `UserConstructionScript`
  (`parent.UserConstructionScript`))