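; Gameplay game mode that spawns the human pawn at a random PlayerSpawnPoint, then places a key fragment away from the player.
; SpawnAKeyFragment steps through KeySpawnPoints, wrapping on the PlayerSpawnPoint count, and rejects those nearer than KeySpawnDistance.
; A rejection sets BadDistance, which Tick uses to retry through a DoOnce until three sections are found.
; The fragment selector is fixed to the first type, and UpdateWaypoint only draws a debug trace to it.
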(event `Update Waypoint`
  ;[1 1 1] Waypoimt System
  (bind _asgameplay_pc (cast `/Game/Blueprints/Gameplay/GameplayPC` (`GameplayStatics.GetPlayerController` 0)))
  (`KismetSystemLibrary.LineTraceSingle` :`Start` (`/Game/Blueprints/Gameplay/GameplayPC.PlayerLocation` _asgameplay_pc) :`End` (`self.KeyLocation`) :`TraceChannel` "TraceTypeQuery1" :`bTraceComplex` true :`DrawDebugType` "Persistent" :`TraceColor` (struct :`G` 1.0 :`B` 0.06713 :`A` 1.0) :`TraceHitColor` (struct :`R` 0.021567 :`G` 1.0 :`A` 1.0)))

(event `self.ReceiveBeginPlay`
  ;[1 0 0.01819] Spawn Player
  (`KismetSystemLibrary.Delay` 1.0)
  (`/Engine/EditorBlueprintResources/StandardMacros.DoOnce` false
    (:`Completed`
      (bind _outactors (`GameplayStatics.GetAllActorsOfClass` "/Game/Spawners/PlayerSpawnPoint.PlayerSpawnPoint_C"))
      (bind _returnvalue (+ (.location (`self.GetTransform` (`|GetArrayItem` _outactors (`KismetMathLibrary.RandomIntegerInRange` 0 (`KismetArrayLibrary.Array_Length` _outactors))))) (0.0 0.0 100.0)))
      (set `self.PlayerSpawnerCoord` _returnvalue)
      (bind _returnvalue_2 (`|SpawnActorFromClass` "/Game/Blueprints/Characters/0_Base_Human.0_Base_Human_C" (`KismetMathLibrary.MakeTransform` _returnvalue (.rotation (`self.GetTransform` (`|GetArrayItem` _outactors (`KismetMathLibrary.RandomIntegerInRange` 0 (`KismetArrayLibrary.Array_Length` _outactors)))))) "AlwaysSpawn" "OverrideRootScale" null null))
      (`Pawn.SpawnDefaultController` _returnvalue_2)
      (`self.EnableInput` _returnvalue_2 (`GameplayStatics.GetPlayerController` 0))
      (`KismetSystemLibrary.Delay` 1.0)
      (`self.Spawn A Key Fragment`))))

(event `Spawn A Key Fragment`
  ;[1 0.815 0] Spawn Key Fragment
  (if (not (== (`self.KeySectionsFound`) 3))
    (set `self.BadDistance` false :!label _label)
    (bind _outactors (`GameplayStatics.GetAllActorsOfClass` "/Game/Spawners/PlayerSpawnPoint.PlayerSpawnPoint_C"))
    (bind _output_get (set `self.SpawnPointNumber` (+ (`self.SpawnPointNumber`) 1)))
    (if (> _output_get (`KismetArrayLibrary.Array_Length` _outactors))
      (set `self.SpawnPointNumber` 0))
    (bind _asgameplay_pc (cast `/Game/Blueprints/Gameplay/GameplayPC` (`GameplayStatics.GetPlayerController` 0))
      (:`then`
        (bind _outactors_2 (`GameplayStatics.GetAllActorsOfClass` "/Game/Spawners/KeySpawnPoint.KeySpawnPoint_C"))
        (bind _outhit (`KismetSystemLibrary.LineTraceSingle` :`Start` (`/Game/Blueprints/Gameplay/GameplayPC.PlayerLocation` _asgameplay_pc) :`End` (.location (`self.GetTransform` (`|GetArrayItem` _outactors_2 (`self.SpawnPointNumber`)))) :`TraceChannel` "TraceTypeQuery1" :`bTraceComplex` true :`DrawDebugType` "Persistent" :`TraceHitColor` (struct :`R` 1.0 :`G` 0.014146 :`A` 1.0)))
        (bind (_bblockinghit _binitialoverlap _time _distance _location _impactpoint _normal _impactnormal _physmat _hitactor _hitcomponent _hitbonename _hititem _faceindex _tracestart _traceend) (`GameplayStatics.BreakHitResult` _outhit))
        (set `self.KeyLocation` _traceend)
        (bind _returnvalue (`KismetMathLibrary.GetPointDistanceToLine` _tracestart _traceend))
        (`KismetSystemLibrary.PrintString` (`KismetStringLibrary.Conv_DoubleToString` _returnvalue) true true (struct :`R` 0.320902 :`B` 1.0 :`A` 1.0))
        (if (< _returnvalue (`self.KeySpawnDistance`))
          (`KismetSystemLibrary.PrintString` "Determining A Key Loccation" true true (struct :`R` 1.0 :`G` 0.200192 :`A` 1.0))
          (`KismetSystemLibrary.RetriggerableDelay` 0.1)
          (set `self.BadDistance` true)
          (else
            (bind _output_get_2 (set `self.KeyFragment` (select `int` 0 :`0` "/Game/Meshes/FragmentedExitKey/KeyFragment1_BP.KeyFragment1_BP_C" :`1` "/Game/Meshes/FragmentedExitKey/KeyFragment2_BP2.KeyFragment2_BP2_C" :`2` "/Game/Meshes/FragmentedExitKey/KeyFragment3_BP3.KeyFragment3_BP3_C" :!type "Actor Class Reference")))
            (`|SpawnActorFromClass` _output_get_2 (`KismetMathLibrary.MakeTransform` _traceend (.rotation (`self.GetTransform` (`|GetArrayItem` _outactors_2 (`self.SpawnPointNumber`))))) "AdjustIfPossibleButAlwaysSpawn" "OverrideRootScale" null null)
            (`KismetSystemLibrary.PrintString` "Key Location Determined" true true (struct :`G` 0.66 :`B` 1.0 :`A` 1.0) 5.0)
            (`self.Update Waypoint`))))
      (:`CastFailed`
        (`KismetSystemLibrary.PrintString` "Cast to Player Controller has failed" true true (struct :`R` 1.0 :`G` 0.00834 :`A` 1.0))))))

(event `Spawn Key`
  ;[1 0.815 0] Spawn Key Fragment
  (if (`self.BadDistance`)
    (if (not (== (`self.KeySectionsFound`) 3))
      (`/Engine/EditorBlueprintResources/StandardMacros.DoOnce` false :!label _label_2
        (:`Completed`
          (goto _label))))
    (else
      (goto _label_2 :!via `Reset`))))

(event `self.ReceiveTick`
  (params (DeltaSeconds :type "Float (single-precision)"))
  ;[1 1 1] Tick Chain
  (`self.Spawn Key`))

(fn `UserConstructionScript`)