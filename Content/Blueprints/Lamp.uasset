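; Lamp Blueprint whose light brightness follows a Sanity value and flickers when it runs low.
; Tick uses a Delay to update the lamp about once a second, scaling intensity by Sanity and Maxintensity, then clamps negative Sanity to zero.
; Below a fifth of maximum intensity, a Flicker timeline drives the light instead.
; Radius overlap and ActiveUtil only set flags, which nothing here reads; Sanity is never decreased here.
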(event `self.ReceiveTick`
  (params (DeltaSeconds :type "Float (single-precision)"))
  ;[1 1 1] Update function
  (`KismetSystemLibrary.Delay` 1.0)
  (`self.UpdateLampStatues`)
  (if (< (`self.Sanity`) 0.0)
    (set `self.Sanity` 0.0)))

(event `UpdateLampStatues`
  ;[1 1 1] Update the lamp
  (if (< (`LightComponentBase.Intensity` (`self.LampLight`)) (* (/ (`self.Maxintensity`) 100.0) 20.0))
    (bind (_direction _flicker) (`Timeline|flicker`)
      (:`Update`
        (`LightComponent.SetIntensity` (`self.LampLight`) (* _flicker 5.0))))
    (else
      (`LightComponent.SetIntensity` (`self.LampLight`) (* (- (`self.Maxintensity`) (* (/ (`self.Maxintensity`) 100.0) 1.0)) (`self.Sanity`)))
      (`KismetSystemLibrary.PrintString` (`KismetStringLibrary.Conv_DoubleToString` (`self.Sanity`))))))

(event `self.ReceiveBeginPlay`
  ;[1 1 1] Event Begin Play
  (`LightComponent.SetIntensity` (`self.LampLight`) (`self.Maxintensity`)))

(event `self.Radius.OnComponentBeginOverlap`
  (params (OverlappedComponent :type "PrimitiveComponent Object Reference") (OtherActor :type "Actor Object Reference") (OtherComp :type "PrimitiveComponent Object Reference") (OtherBodyIndex :type Integer) (bFromSweep :type Boolean) (SweepResult :type "HitResult Structure (by ref)"))
  ;[1 0.3245 0.5163] Collision area being overlapped
  (set `self.Overlapped` true))

(fn `Active_Util`
  (params (Flag :type Boolean))
  (set `self.Active` Flag))

(fn `UserConstructionScript`)