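; WaypointNode is a waypoint actor that appears to be a work-in-progress part of a waypoint system.
; Every tick it turns its Arrow toward the player character, marked as testing only.
; When a 0_Base_Human enters DetectionZone, it clears WaypointSelection on the third WaypointNode found, then debug-draws a visibility multi-trace toward that just-cleared selection.
; The trace results are unused.
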(event `Rotate to Face Player`
  (bind _arrow (`self.Arrow`))
  ;[0 0.6546 1] Face Waypoint in player Direction (Only necessary for testing)
  (`SceneComponent.K2_SetWorldRotation` _arrow (`KismetMathLibrary.FindLookAtRotation` (`SceneComponent.K2_GetComponentLocation` _arrow) (`self.K2_GetActorLocation` (`GameplayStatics.GetPlayerCharacter` 0))) false false))

(event `self.ReceiveTick`
  (params (DeltaSeconds :type "Float (single-precision)"))
  ;[1 1 1] Tick Chain
  (`self.Rotate to Face Player`))

(event `self.DetectionZone.OnComponentBeginOverlap`
  (params (OverlappedComponent :type "PrimitiveComponent Object Reference") (OtherActor :type "Actor Object Reference") (OtherComp :type "PrimitiveComponent Object Reference") (OtherBodyIndex :type Integer) (bFromSweep :type Boolean) (SweepResult :type "HitResult Structure (by ref)"))
  (bind _as0_base_human (cast `/Game/Blueprints/Characters/0_Base_Human` OtherActor))
  (bind _outactors (`GameplayStatics.GetAllActorsOfClass` "WaypointNode_C"))
  (bind _output_get (set `/Game/Blueprints/WaypointSystem/WaypointNode.WaypointSelection` null (`|GetArrayItem` _outactors 2)))
  (`KismetSystemLibrary.LineTraceMulti` :`Start` (`self.K2_GetActorLocation`) :`End` (`self.K2_GetActorLocation` _output_get) :`TraceChannel` "TraceTypeQuery1" :`bTraceComplex` true :`DrawDebugType` "Persistent" :`TraceColor` (struct :`G` 0.824866 :`B` 1.0 :`A` 1.0) :`TraceHitColor` (struct :`G` 0.314345 :`B` 1.0 :`A` 1.0)))

(fn `UserConstructionScript`)